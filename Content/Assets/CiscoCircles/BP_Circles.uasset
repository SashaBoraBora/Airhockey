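; BP_Circles is an actor that applies a subtle vertical and roll animation to its Ring1, Ring3 and Ring5 components.
; On BeginPlay it derives small offsets either side of Ring1's world height and roll, then plays a Timeline to interpolate between them.
; All three rings receive the same world location and rotation from Ring1's values, with pitch and yaw forced to zero.
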(event `self.ReceiveBeginPlay`
  (bind _ring_1 (`self.ring_1`))
  (bind _ring_1_2 (`self.ring_1`))
  (bind _returnvalue (`SceneComponent.K2_GetComponentLocation` _ring_1))
  (bind _returnvalue_roll (`KismetMathLibrary.BreakRotator` (`SceneComponent.K2_GetComponentRotation` _ring_1)))
  (bind _output_get (set `self.Start1` (+ _returnvalue (0.0 0.0 -0.5))))
  (bind _output_get_2 (set `self.End1` (+ _returnvalue (0.0 0.0 0.5))))
  (bind _output_get_3 (set `self.StartRotator` (+ _returnvalue_roll -1.0)))
  (bind _output_get_4 (set `self.EndRotator` (+ _returnvalue_roll 1.0)))
  (bind (_direction _newtrack_1) (`Timeline|Timeline`)
    (:`Update`
      (`SceneComponent.K2_SetWorldLocation` _ring_1_2 (`KismetMathLibrary.VLerp` _output_get _output_get_2 _newtrack_1) false false)
      (`SceneComponent.K2_SetWorldLocation` (`self.ring_3`) (`KismetMathLibrary.VLerp` _output_get _output_get_2 _newtrack_1) false false)
      (`SceneComponent.K2_SetWorldLocation` (`self.ring_5`) (`KismetMathLibrary.VLerp` _output_get _output_get_2 _newtrack_1) false false)
      (`SceneComponent.K2_SetWorldRotation` _ring_1_2 (`KismetMathLibrary.MakeRotator` (`KismetMathLibrary.Lerp` _output_get_3 _output_get_4 _newtrack_1)) false false)
      (`SceneComponent.K2_SetWorldRotation` (`self.ring_3`) (`KismetMathLibrary.MakeRotator` (`KismetMathLibrary.Lerp` _output_get_3 _output_get_4 _newtrack_1)) false false)
      (`SceneComponent.K2_SetWorldRotation` (`self.ring_5`) (`KismetMathLibrary.MakeRotator` (`KismetMathLibrary.Lerp` _output_get_3 _output_get_4 _newtrack_1)) false false))))

(fn `UserConstructionScript`)