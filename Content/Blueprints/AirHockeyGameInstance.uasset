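; Game instance for an air hockey game that holds match settings, match time, a marker-use flag and leaderboard submission.
; On Init or Read it loads goal count and power-up time from a JSON settings file in project content.
; A looping timer accumulates match time.
; Per-player events combine entered credentials with that time, append it to the save game, refresh the leaderboard UI, then trigger a delayed JSON save through the JSON manager.
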(event `Read`
  (bind _outjsonobject (`JsonBlueprintFunctionLibrary.FromFile` (make `FilePath` (`KismetStringLibrary.Concat_StrStr` (`KismetSystemLibrary.GetProjectContentDirectory`) "Data/game_settings.json")) :!label _label))
  (bind _output_get (set `self.Json Object` _outjsonobject))
  (bind _outvalue (`|GetJsonField` _output_get "NumberOfGoals"))
  (set `self.NumberOfGoals` _outvalue)
  (bind _outvalue_2 (`|GetJsonField` _output_get "PowerUpTimeInSeconds"))
  (set `self.PowerUpTime` _outvalue_2))

(event `self.ReceiveInit`
  (goto _label))

(event `Count Game Time`
  (bind _returnvalue (`KismetSystemLibrary.K2_SetTimer` null "CountMatchTime" 0.1 true))
  (set `self.HandleMatchTimeCounter` _returnvalue))

(event `StopCountGameTime`
  (`KismetSystemLibrary.K2_ClearAndInvalidateTimerHandle` (`self.HandleMatchTimeCounter`)))

(event `ResetMatchTime`
  (set `self.MatchTime` 0.0))

(event `AddToLeaderboardArrayP1`
  (bind _wp_entercredentials (`/Game/Widget/WB_PlayerBaseUIP1.WP_EnterCredentials` (`/Game/Blueprints/BP_AirhockeyPawn.UIRefP1` (`self.As BP Airhockey Pawn`))))
  (`/Engine/EditorBlueprintResources/StandardMacros.IsValid` (`self.JsonManagerRef`)
    (:`Is Valid`
      _)
    (:`Is Not Valid`
      (bind _returnvalue (`GameplayStatics.GetActorOfClass` "/Game/Blueprints/bp_JSONManager.bp_JSONManager_C"))
      (set `self.JsonManagerRef` _returnvalue)))
  (`/Engine/EditorBlueprintResources/StandardMacros.IsValid` (`self.As BP Airhockey Pawn`)
    (:`Is Valid`
      _)
    (:`Is Not Valid`
      (bind _asbp_airhockey_pawn (cast `/Game/Blueprints/BP_AirhockeyPawn` (`GameplayStatics.GetPlayerPawn` 0)))
      (set `self.As BP Airhockey Pawn` _asbp_airhockey_pawn)))
  (set `self.leaderboardObject` (make `/Game/Blueprints/Struct_Leaderboard` (`KismetTextLibrary.Conv_TextToString` (`/Game/Widget/WP_EnterCredential_P1.NameText` _wp_entercredentials)) (`KismetTextLibrary.Conv_TextToString` (`/Game/Widget/WP_EnterCredential_P1.Surname Text` _wp_entercredentials)) (`self.MatchTime`) (`KismetTextLibrary.Conv_TextToString` (`/Game/Widget/WP_EnterCredential_P1.EmailText` _wp_entercredentials)) (`KismetTextLibrary.Conv_TextToString` (`/Game/Widget/WP_EnterCredential_P1.CompanyText` _wp_entercredentials))))
  (bind _returnvalue_2 (`GameplayStatics.DoesSaveGameExist` "savegame"))
  (if _returnvalue_2
    (bind _returnvalue_3 (`GameplayStatics.LoadGameFromSlot` "savegame"))
    (bind _asbp_leaderboardsavegame (cast `/Game/Blueprints/bp_leaderboardsavegame` _returnvalue_3))
    (`KismetArrayLibrary.Array_AddUnique` (`/Game/Blueprints/bp_leaderboardsavegame.player entries` _asbp_leaderboardsavegame) (`self.leaderboardObject`))
    (`GameplayStatics.SaveGameToSlot` _asbp_leaderboardsavegame "savegame")
    (`/Game/Widget/WB_LeadboardUI.update` (`/Game/Blueprints/BP_AirhockeyPawn.LeaderboardUIRef` (`self.As BP Airhockey Pawn`)))
    (`KismetSystemLibrary.Delay` 2.0)
    (`/Game/Blueprints/bp_JSONManager.SaveJson` (`self.JsonManagerRef`))
    (`KismetSystemLibrary.PrintString` "Hi1")
    (else
      (bind _returnvalue_4 (`GameplayStatics.CreateSaveGameObject` "/Game/Blueprints/bp_leaderboardsavegame.bp_leaderboardsavegame_C"))
      (`KismetArrayLibrary.Array_AddUnique` (`/Game/Blueprints/bp_leaderboardsavegame.player entries` _returnvalue_4) (`self.leaderboardObject`))
      (`GameplayStatics.SaveGameToSlot` _returnvalue_4 "savegame")
      (`/Game/Widget/WB_LeadboardUI.update` (`/Game/Blueprints/BP_AirhockeyPawn.LeaderboardUIRef` (`self.As BP Airhockey Pawn`)))
      (`KismetSystemLibrary.Delay` 2.0)
      (`/Game/Blueprints/bp_JSONManager.SaveJson` (`self.JsonManagerRef`))
      (`KismetSystemLibrary.PrintString` "Hi2"))))

(event `AddToLeaderboardArrayP2`
  (bind _wpentercredentials (`/Game/Widget/WB_PlayerBaseUIP2.WPEnterCredentials` (`/Game/Blueprints/BP_AirhockeyPawn.UIRefP2` (`self.As BP Airhockey Pawn`))))
  (`/Engine/EditorBlueprintResources/StandardMacros.IsValid` (`self.JsonManagerRef`)
    (:`Is Valid`
      _)
    (:`Is Not Valid`
      (bind _returnvalue (`GameplayStatics.GetActorOfClass` "/Game/Blueprints/bp_JSONManager.bp_JSONManager_C"))
      (set `self.JsonManagerRef` _returnvalue)))
  (`/Engine/EditorBlueprintResources/StandardMacros.IsValid` (`self.As BP Airhockey Pawn`)
    (:`Is Valid`
      _)
    (:`Is Not Valid`
      (bind _asbp_airhockey_pawn (cast `/Game/Blueprints/BP_AirhockeyPawn` (`GameplayStatics.GetPlayerPawn` 0)))
      (set `self.As BP Airhockey Pawn` _asbp_airhockey_pawn)))
  (set `self.leaderboardObject` (make `/Game/Blueprints/Struct_Leaderboard` (`KismetTextLibrary.Conv_TextToString` (`/Game/Widget/WP_EnterCredential_P2.NameText` _wpentercredentials)) (`KismetTextLibrary.Conv_TextToString` (`/Game/Widget/WP_EnterCredential_P2.Surname Text` _wpentercredentials)) (`self.MatchTime`) (`KismetTextLibrary.Conv_TextToString` (`/Game/Widget/WP_EnterCredential_P2.EmailText` _wpentercredentials)) (`KismetTextLibrary.Conv_TextToString` (`/Game/Widget/WP_EnterCredential_P2.CompanyText` _wpentercredentials))))
  (bind _returnvalue_2 (`GameplayStatics.DoesSaveGameExist` "savegame"))
  (if _returnvalue_2
    (bind _returnvalue_3 (`GameplayStatics.LoadGameFromSlot` "savegame"))
    (bind _asbp_leaderboardsavegame (cast `/Game/Blueprints/bp_leaderboardsavegame` _returnvalue_3))
    (`KismetArrayLibrary.Array_AddUnique` (`/Game/Blueprints/bp_leaderboardsavegame.player entries` _asbp_leaderboardsavegame) (`self.leaderboardObject`))
    (`GameplayStatics.SaveGameToSlot` _asbp_leaderboardsavegame "savegame")
    (`/Game/Widget/WB_LeadboardUI.update` (`/Game/Blueprints/BP_AirhockeyPawn.LeaderboardUIRef` (`self.As BP Airhockey Pawn`)))
    (`KismetSystemLibrary.Delay` 2.0)
    (`/Game/Blueprints/bp_JSONManager.SaveJson` (`self.JsonManagerRef`))
    (`KismetSystemLibrary.PrintString` "Hi3")
    (else
      (bind _returnvalue_4 (`GameplayStatics.CreateSaveGameObject` "/Game/Blueprints/bp_leaderboardsavegame.bp_leaderboardsavegame_C"))
      (`KismetArrayLibrary.Array_AddUnique` (`/Game/Blueprints/bp_leaderboardsavegame.player entries` _returnvalue_4) (`self.leaderboardObject`))
      (`GameplayStatics.SaveGameToSlot` _returnvalue_4 "savegame")
      (`/Game/Widget/WB_LeadboardUI.update` (`/Game/Blueprints/BP_AirhockeyPawn.LeaderboardUIRef` (`self.As BP Airhockey Pawn`)))
      (`KismetSystemLibrary.Delay` 2.0)
      (`/Game/Blueprints/bp_JSONManager.SaveJson` (`self.JsonManagerRef`))
      (`KismetSystemLibrary.PrintString` "Hi4"))))

(event `SetUserMarkerTrue`
  (set `self.UseMarker` true))

(event `SetUseMarkerFalse`
  (set `self.UseMarker` false))

(fn `CountMatchTime`
  (set `self.MatchTime` (+ (`self.MatchTime`) 0.1)))