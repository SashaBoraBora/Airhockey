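; Air hockey touch tracker that moves Player 1's paddle on the pawn when touch-triangle angles match a stored paddle angle.
; Each Tick samples touches 1–3 and computes corner angles for triangles ABC and DEF, though DEF points are only self-assigned.
; Each angle within threshold of Paddle1A triggers screen-to-world traces and a circumcenter-based paddle move.
; All three traces use the same touch point, so the circumcenter receives identical inputs.
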(event `self.ReceiveBeginPlay`
  (bind _asbp_airhockey_pawn (cast `/Game/Blueprints/BP_AirhockeyPawn` (`GameplayStatics.GetPlayerPawn` 0)))
  (set `self.As BP Airhockey Pawn` _asbp_airhockey_pawn))

(event `self.ReceiveTick`
  (params (DeltaSeconds :type "Float (single-precision)"))
  (bind _returnvalue (`GameplayStatics.GetPlayerController` 0))
  (bind _threshold (`self.Threshold`))
  (bind _paddle_1a (`self.Paddle_1A`))
  (bind _threshold_2 (`self.Threshold`))
  (bind _paddle_1a_2 (`self.Paddle_1A`))
  (bind _threshold_3 (`self.Threshold`))
  (bind _paddle_1a_3 (`self.Paddle_1A`))
  (`|ExecutionSequence`
    (:`then_0`
      (`self.Update Touch Points`))
    (:`then_1`
      (bind _output_get (set `self.TouchPointA` (`self.LocalTouchA`)))
      (bind _output_get_2 (set `self.TouchPointB` (`self.LocalTouchB`)))
      (bind _output_get_3 (set `self.TouchPointC` (`self.LocalTouchC`)))
      (bind _output_get_4 (set `self.TouchPointD` (`self.TouchPointD`)))
      (bind _output_get_5 (set `self.TouchPointE` (`self.TouchPointE`)))
      (bind _output_get_6 (set `self.TouchPointF` (`self.TouchPointF`)))
      (set `self.TouchPointArray` (`|MakeArray` _output_get _output_get_2 _output_get_3 _output_get_4 _output_get_5 _output_get_6)))
    (:`then_2`
      (bind (_winkela _winkelb _winkelc) (`self.Calculate Angles ABC`))
      (bind (_winkeld _winkele _winkelf) (`self.Calculate Angles DEF`))
      (set `self.AngleArray` (`|MakeArray` _winkela _winkelb _winkelc _winkeld _winkele _winkelf)))
    (:`then_3`
      (for (_array_element _array_index) (`self.AngleArray`)
        (if (and (`KismetMathLibrary.InRange_FloatFloat` _array_element (- _paddle_1a _threshold_2) (+ _paddle_1a _threshold_2)) (`KismetMathLibrary.InRange_FloatFloat` _array_element (- _paddle_1a_2 _threshold_3) (+ _paddle_1a_2 _threshold_3)) (`KismetMathLibrary.InRange_FloatFloat` _array_element (- _paddle_1a_3 _threshold) (+ _paddle_1a_3 _threshold)))
          (bind (_output_x _output_y) (`KismetMathLibrary.BreakVector2D` (`|GetArrayItem` (`self.TouchPointArray`) _array_index)))
          (bind (_worldlocation _worlddirection) (`PlayerController.DeprojectScreenPositionToWorld` _returnvalue _output_x _output_y))
          (bind _outhit (`KismetSystemLibrary.LineTraceSingle` _worldlocation (+ _worldlocation (* _worlddirection 10000.0)) "TraceTypeQuery1"))
          (bind (_output_x_2 _output_y_2) (`KismetMathLibrary.BreakVector2D` (`|GetArrayItem` (`self.TouchPointArray`) _array_index)))
          (bind (_worldlocation_2 _worlddirection_2) (`PlayerController.DeprojectScreenPositionToWorld` _returnvalue _output_x_2 _output_y_2))
          (bind _outhit_2 (`KismetSystemLibrary.LineTraceSingle` _worldlocation_2 (+ _worldlocation_2 (* _worlddirection_2 10000.0)) "TraceTypeQuery1"))
          (bind (_output_x_3 _output_y_3) (`KismetMathLibrary.BreakVector2D` (`|GetArrayItem` (`self.TouchPointArray`) _array_index)))
          (bind (_worldlocation_3 _worlddirection_3) (`PlayerController.DeprojectScreenPositionToWorld` _returnvalue _output_x_3 _output_y_3))
          (bind _outhit_3 (`KismetSystemLibrary.LineTraceSingle` _worldlocation_3 (+ _worldlocation_3 (* _worlddirection_3 10000.0)) "TraceTypeQuery1"))
          (bind _outcircumcenter (`MyBlueprintFunctionLibrary.CalculateCircumcenter` (`.Location` (`GameplayStatics.BreakHitResult` _outhit)) (`.Location` (`GameplayStatics.BreakHitResult` _outhit_2)) (`.Location` (`GameplayStatics.BreakHitResult` _outhit_3))))
          (bind _output_get_7 (set `self.Out Circumcenter X` (.x _outcircumcenter)))
          (bind _output_get_8 (set `self.Out Circumcenter Y` (.y _outcircumcenter)))
          (`SceneComponent.K2_SetWorldLocation` (`/Game/Blueprints/BP_AirhockeyPawn.Player1Paddle` (`self.As BP Airhockey Pawn`)) (`KismetMathLibrary.MakeVector` _output_get_7 _output_get_8 10.0) true false)
          (else
            (`KismetSystemLibrary.PrintString` "Hello")))))))

(fn `Calculate Angles ABC`
  (returns (WinkelA :type "Float (double-precision)") (WinkelB :type "Float (double-precision)") (WinkelC :type "Float (double-precision)"))
  (bind _output_get (set `self.AB` (- (`self.TouchPointB`) (`self.TouchPointA`))))
  (bind _output_get_2 (set `self.AC` (- (`self.TouchPointC`) (`self.TouchPointA`))))
  (bind _output_get_3 (set `self.BC` (- (`self.TouchPointC`) (`self.TouchPointB`))))
  (return (`KismetMathLibrary.DegAcos` (/ (`KismetMathLibrary.DotProduct2D` _output_get _output_get_2) (* (`KismetMathLibrary.VSize2D` (`self.AB`)) (`KismetMathLibrary.VSize2D` (`self.AC`))))) (`KismetMathLibrary.DegAcos` (/ (`KismetMathLibrary.DotProduct2D` (* _output_get -1.0) _output_get_3) (* (`KismetMathLibrary.VSize2D` (`self.AB`)) (`KismetMathLibrary.VSize2D` (`self.BC`))))) (`KismetMathLibrary.DegAcos` (/ (`KismetMathLibrary.DotProduct2D` (* _output_get_2 -1.0) (* _output_get_3 -1.0)) (* (`KismetMathLibrary.VSize2D` (`self.AC`)) (`KismetMathLibrary.VSize2D` (`self.BC`)))))))

(fn `Calculate Angles DEF`
  (returns (WinkelD :type "Float (double-precision)") (WinkelE :type "Float (double-precision)") (WinkelF :type "Float (double-precision)"))
  (bind _output_get (set `self.DE` (- (`self.TouchPointE`) (`self.TouchPointD`))))
  (bind _output_get_2 (set `self.DF` (- (`self.TouchPointF`) (`self.TouchPointD`))))
  (bind _output_get_3 (set `self.EF` (- (`self.TouchPointF`) (`self.TouchPointE`))))
  (return (`KismetMathLibrary.DegAcos` (/ (`KismetMathLibrary.DotProduct2D` _output_get _output_get_2) (* (`KismetMathLibrary.VSize2D` (`self.DE`)) (`KismetMathLibrary.VSize2D` (`self.DF`))))) (`KismetMathLibrary.DegAcos` (/ (`KismetMathLibrary.DotProduct2D` (* _output_get -1.0) _output_get_3) (* (`KismetMathLibrary.VSize2D` (`self.DE`)) (`KismetMathLibrary.VSize2D` (`self.EF`))))) (`KismetMathLibrary.DegAcos` (/ (`KismetMathLibrary.DotProduct2D` (* _output_get_2 -1.0) (* _output_get_3 -1.0)) (* (`KismetMathLibrary.VSize2D` (`self.DF`)) (`KismetMathLibrary.VSize2D` (`self.EF`)))))))

(fn `Update Touch Points`
  (bind (_locationx _locationy) (`PlayerController.GetInputTouchState` (`GameplayStatics.GetPlayerController` 0) "Touch1"))
  (bind (_locationx_2 _locationy_2) (`PlayerController.GetInputTouchState` (`GameplayStatics.GetPlayerController` 0) "Touch2"))
  (bind (_locationx_3 _locationy_3) (`PlayerController.GetInputTouchState` (`GameplayStatics.GetPlayerController` 0) "Touch1"))
  (bind (_locationx_4 _locationy_4) (`PlayerController.GetInputTouchState` (`GameplayStatics.GetPlayerController` 0) "Touch2"))
  (bind (_locationx_5 _locationy_5) (`PlayerController.GetInputTouchState` (`GameplayStatics.GetPlayerController` 0) "Touch3"))
  (bind (_locationx_6 _locationy_6) (`PlayerController.GetInputTouchState` (`GameplayStatics.GetPlayerController` 0) "Touch3"))
  (set `self.LocalTouchA` (`KismetMathLibrary.MakeVector2D` _locationx _locationy))
  (set `self.LocalTouchB` (`KismetMathLibrary.MakeVector2D` _locationx_2 _locationy_2))
  (set `self.LocalTouchC` (`KismetMathLibrary.MakeVector2D` _locationx_6 _locationy_6))
  (set `self.LocalTouchD` (`KismetMathLibrary.MakeVector2D` _locationx_3 _locationy_3))
  (set `self.LocalTouchE` (`KismetMathLibrary.MakeVector2D` _locationx_4 _locationy_4))
  (set `self.LocalTouchF` (`KismetMathLibrary.MakeVector2D` _locationx_5 _locationy_5)))

(fn `UserConstructionScript`)