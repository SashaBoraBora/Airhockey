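; BP_P1_HybridMeshFirewall is a Player 1 firewall power in an air hockey game, made of attached segment actors.
; On BeginPlay, if the player pawn is BP_AirhockeyPawn, a timeline scales the segments up from zero and records their count.
; DestroyPowerP1 scales them down on a second timeline and destroys the firewall after a short delay.
; Decrement lowers the segment count and destroys the firewall when it reaches zero.
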(event `self.ReceiveBeginPlay`
  (bind _asbp_airhockey_pawn (cast `/Game/Blueprints/BP_AirhockeyPawn` (`GameplayStatics.GetPlayerPawn` 0)))
  (set `self.As BP Airhockey Pawn` _asbp_airhockey_pawn)
  (bind (_direction _newtrack_0) (`Timeline|Timeline_0`)
    (:`Update`
      (for _array_element (`self.GetAttachedActors` true)
        (`self.SetActorRelativeScale3D` _array_element (`KismetMathLibrary.VLerp` (0.0 0.0 0.0) (1.0 1.0 1.0) _newtrack_0))
        (set `self.RemainingSegments` (`KismetArrayLibrary.Array_Length` (`self.GetAttachedActors` true)))))))

(event `/Game/Blueprints/BI_GamestartCisco.DestroyPowerP1`
  (bind (_direction _newtrack_0) (`Timeline|Timeline` :!via `PlayFromStart`)
    (:`Update`
      (for _array_element (`self.GetAttachedActors` true)
        (`self.SetActorRelativeScale3D` _array_element (`KismetMathLibrary.VLerp` (1.0 1.0 1.0) (0.0 0.0 0.0) _newtrack_0))
        (`KismetSystemLibrary.Delay` 0.25)
        (`self.K2_DestroyActor`)))))

(event `Decrement`
  (`/Engine/EditorBlueprintResources/StandardMacros.DecrementInt` (`self.RemainingSegments`)
    (:`  `
      (if (== (`self.RemainingSegments`) 0)
        (`KismetSystemLibrary.PrintString` "Destroyed")
        (`self.K2_DestroyActor`)
        (else
          (`KismetSystemLibrary.PrintString` "NotDestroyed"))))))

(fn `UserConstructionScript`)