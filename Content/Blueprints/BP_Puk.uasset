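; BP_Puk is a physics-simulated mesh actor, apparently a puck, that plays hit sounds on contact.
; On BeginPlay it turns physics off, then re-enables it after a short delay.
; Any overlap with its Sphere component plays one of four random sounds at the world origin rather than at the mesh.
; A PlayHitSound tag check and a mesh location lookup exist but are left unconnected.
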(event `self.ReceiveBeginPlay`
  (`PrimitiveComponent.SetSimulatePhysics` (`self.StaticMesh`) false)
  (`KismetSystemLibrary.Delay` 0.2)
  (`PrimitiveComponent.SetSimulatePhysics` (`self.StaticMesh`) true))

(event `self.Sphere.OnComponentBeginOverlap`
  (params (OverlappedComponent :type "PrimitiveComponent Object Reference") (OtherActor :type "Actor Object Reference") (OtherComp :type "PrimitiveComponent Object Reference") (OtherBodyIndex :type Integer) (bFromSweep :type Boolean) (SweepResult :type "HitResult Structure (by ref)"))
  (`GameplayStatics.PlaySoundAtLocation` (`|GetArrayItem` (`self.Sound`) (`KismetMathLibrary.RandomIntegerInRange` 0 3)) (0.0 0.0 0.0) (struct) 1.0 1.0 0.0 null null null null))

(event `self.ReceiveTick`
  (params (DeltaSeconds :type "Float (single-precision)")))

(fn `UserConstructionScript`)