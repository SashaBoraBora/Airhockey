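; Air hockey table sides actor that detects goals and updates the score.
; Two overlap components react to BP_Puk: Player scores for the AI and Goal scores for the player, through HUD widgets on the cached BP_AirhockeyPawn.
; Each goal hides the puck, disables its physics and moves it to table center, then restores both after a short delay.
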(event `self.ReceiveBeginPlay`
  (bind _asbp_airhockey_pawn (cast `/Game/Blueprints/BP_AirhockeyPawn` (`GameplayStatics.GetPlayerPawn` 0)))
  (set `self.As BP Airhockey Pawn` _asbp_airhockey_pawn))

(event `self.Player.OnComponentBeginOverlap`
  (params (OverlappedComponent :type "PrimitiveComponent Object Reference") (OtherActor :type "Actor Object Reference") (OtherComp :type "PrimitiveComponent Object Reference") (OtherBodyIndex :type Integer) (bFromSweep :type Boolean) (SweepResult :type "HitResult Structure (by ref)"))
  (bind _asbp_puk (cast `/Game/Blueprints/BP_Puk` OtherActor))
  (bind _staticmesh (`/Game/Blueprints/BP_Puk.StaticMesh` _asbp_puk))
  (`SceneComponent.SetHiddenInGame` _staticmesh true false)
  (`PrimitiveComponent.SetSimulatePhysics` _staticmesh false)
  (`/Game/Widget/WB_ScoreCountAI.AddToScoreAI` (`/Game/Widget/WB_HUD.WB_ScoreCountAI` (`/Game/Blueprints/BP_AirhockeyPawn.HUDRef` (`self.As BP Airhockey Pawn`))))
  (`SceneComponent.K2_SetWorldLocation` _staticmesh (0.0 0.0 11.191809) false false)
  (`KismetSystemLibrary.Delay` 0.5)
  (`SceneComponent.SetHiddenInGame` _staticmesh false false)
  (`PrimitiveComponent.SetSimulatePhysics` _staticmesh true))

(event `self.Goal.OnComponentBeginOverlap`
  (params (OverlappedComponent :type "PrimitiveComponent Object Reference") (OtherActor :type "Actor Object Reference") (OtherComp :type "PrimitiveComponent Object Reference") (OtherBodyIndex :type Integer) (bFromSweep :type Boolean) (SweepResult :type "HitResult Structure (by ref)"))
  (bind _asbp_puk (cast `/Game/Blueprints/BP_Puk` OtherActor))
  (bind _staticmesh (`/Game/Blueprints/BP_Puk.StaticMesh` _asbp_puk))
  (`SceneComponent.SetHiddenInGame` _staticmesh true false)
  (`PrimitiveComponent.SetSimulatePhysics` _staticmesh false)
  (`/Game/Widget/WB_ScoreCountPlayer.AddToScorePlayer` (`/Game/Widget/WB_HUD.WB_ScoreCount` (`/Game/Blueprints/BP_AirhockeyPawn.HUDRef` (`self.As BP Airhockey Pawn`))))
  (`SceneComponent.K2_SetWorldLocation` _staticmesh (0.0 0.0 11.191809) false false)
  (`KismetSystemLibrary.Delay` 0.5)
  (`SceneComponent.SetHiddenInGame` _staticmesh false false)
  (`PrimitiveComponent.SetSimulatePhysics` _staticmesh true))

(fn `UserConstructionScript`)