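; BP_MenuPawn is the starting pawn for the air hockey game's menu, handing off to the gameplay pawn.
; On BeginPlay it caches the air hockey player controller, spawns BP_AirhockeyPawn at a fixed transform, and has the player controller possess the menu pawn.
; Pressing the 2 key asks the controller to blend the camera to the hockey pawn, then possesses it after a delay slightly longer than the blend.
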(event `self.ReceiveBeginPlay`
  (bind _asbp_player_controller_airhockey (cast `/Game/Blueprints/BP_PlayerControllerAirhockey` (`GameplayStatics.GetPlayerController` 0)))
  (set `self.PlayerControllerRef` _asbp_player_controller_airhockey)
  (bind _returnvalue (`|SpawnActorFromClass` "/Game/Blueprints/BP_AirhockeyPawn.BP_AirhockeyPawn_C" (`KismetMathLibrary.MakeTransform` (0.0 0.0 190.0) (struct :`Yaw` -90.0)) "Undefined" "MultiplyWithRoot" null null))
  (set `self.AirHockeyPawnRef` _returnvalue)
  (`Controller.Possess` (`GameplayStatics.GetPlayerController` 0) self))

(event `Key|Two`
  (params (Key :type "Key Structure"))
  (:`Pressed`
    (`/Game/Blueprints/BP_PlayerControllerAirhockey.MoveCameraTo` (`self.PlayerControllerRef`) (`self.AirHockeyPawnRef`) 2.0)
    (`KismetSystemLibrary.Delay` 3.0)
    (`Controller.Possess` (`GameplayStatics.GetPlayerController` 0) (`self.AirHockeyPawnRef`))))

(fn `UserConstructionScript`)