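; BP_FakePucks is a physics-simulated fake puck in the air hockey game that removes itself when the active power is destroyed.
; On BeginPlay it casts player pawn 0 to BP_AirhockeyPawn and binds to the DestroyPower dispatcher on its UI's active power widget.
; That event plays a Timeline that shrinks the puck toward zero scale, with a short Delay from the update pin before destroying the actor.
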(event `self.ReceiveBeginPlay`
  (bind _asbp_airhockey_pawn (cast `/Game/Blueprints/BP_AirhockeyPawn` (`GameplayStatics.GetPlayerPawn` 0)))
  (set `self.As BP Airhockey Pawn` _asbp_airhockey_pawn)
  (`PrimitiveComponent.SetSimulatePhysics` (`self.StaticMesh`) true)
  (add `/Game/Widget/WB_ActivePower.DestroyPower` (`/Game/Widget/WB_PlayerBaseUI.WB_ActivePower` (`/Game/Blueprints/BP_AirhockeyPawn.UIRef` (`self.As BP Airhockey Pawn`))) (delegate `DestroyPower_Event`)))

(event `DestroyPower_Event`
  (bind (_direction _newtrack_0) (`Timeline|Timeline`)
    (:`Update`
      (`self.SetActorRelativeScale3D` (`KismetMathLibrary.VLerp` (0.2 0.2 0.2) (0.0 0.0 0.0) _newtrack_0))
      (`KismetSystemLibrary.Delay` 0.25)
      (`self.K2_DestroyActor`))))

(fn `UserConstructionScript`)