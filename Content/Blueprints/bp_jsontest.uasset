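; Test actor that saves air hockey players' entered credentials to a JSON file, then restarts the game.
; Separate P1 and P2 events read name, surname, email and company from that player's UI on the cached pawn, with a placeholder time.
; Both write to the same test.json, wait, close all multi-window extension windows and open AirhockeyMain.
; An unfinished load-and-merge branch is never run.
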(event `self.ReceiveBeginPlay`
  (bind _asbp_airhockey_pawn (cast `/Game/Blueprints/BP_AirhockeyPawn` (`GameplayStatics.GetPlayerPawn` 0)))
  (set `self.As BP Airhockey Pawn` _asbp_airhockey_pawn))

(event `saveJsonP1`
  (bind _wp_entercredentials (`/Game/Widget/WB_PlayerBaseUIP1.WP_EnterCredentials` (`/Game/Blueprints/BP_AirhockeyPawn.UIRefP1` (`self.As BP Airhockey Pawn`))))
  (bind _returnvalue (`VaRestJsonObject.WriteToFilePath` (`|MakeJson` (`KismetTextLibrary.Conv_TextToString` (`/Game/Widget/WP_EnterCredential_P1.NameText` _wp_entercredentials)) (`KismetTextLibrary.Conv_TextToString` (`/Game/Widget/WP_EnterCredential_P1.Surname Text` _wp_entercredentials)) "0000" (`KismetTextLibrary.Conv_TextToString` (`/Game/Widget/WP_EnterCredential_P1.EmailText` _wp_entercredentials)) (`KismetTextLibrary.Conv_TextToString` (`/Game/Widget/WP_EnterCredential_P1.CompanyText` _wp_entercredentials))) "Content/Data/test.json" true))
  (`KismetSystemLibrary.PrintString` (`KismetStringLibrary.Conv_BoolToString` _returnvalue))
  (`KismetSystemLibrary.Delay` 5.0)
  (`MultiWindowExtensionSubsystem.KB_MWE_CloseAll` (subsystem `MultiWindowExtensionSubsystem`))
  (`KismetSystemLibrary.Delay` 0.1)
  (`GameplayStatics.OpenLevel` "AirhockeyMain"))

(event `saveJsonP2`
  (bind _wpentercredentials (`/Game/Widget/WB_PlayerBaseUIP2.WPEnterCredentials` (`/Game/Blueprints/BP_AirhockeyPawn.UIRefP2` (`self.As BP Airhockey Pawn`))))
  (bind _returnvalue (`VaRestJsonObject.WriteToFilePath` (`|MakeJson` (`KismetTextLibrary.Conv_TextToString` (`/Game/Widget/WP_EnterCredential_P2.NameText` _wpentercredentials)) (`KismetTextLibrary.Conv_TextToString` (`/Game/Widget/WP_EnterCredential_P2.Surname Text` _wpentercredentials)) "0000" (`KismetTextLibrary.Conv_TextToString` (`/Game/Widget/WP_EnterCredential_P2.EmailText` _wpentercredentials)) (`KismetTextLibrary.Conv_TextToString` (`/Game/Widget/WP_EnterCredential_P2.CompanyText` _wpentercredentials))) "Content/Data/test.json" true))
  (`KismetSystemLibrary.PrintString` (`KismetStringLibrary.Conv_BoolToString` _returnvalue))
  (`KismetSystemLibrary.Delay` 5.0)
  (`MultiWindowExtensionSubsystem.KB_MWE_CloseAll` (subsystem `MultiWindowExtensionSubsystem`))
  (`KismetSystemLibrary.Delay` 0.1)
  (`GameplayStatics.OpenLevel` "AirhockeyMain"))

(fn `UserConstructionScript`)