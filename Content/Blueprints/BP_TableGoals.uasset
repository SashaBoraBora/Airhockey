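; Air hockey table goals actor that handles scoring, win checks and the Splunk goal-resizing power for both players.
; Goal overlaps with the puck or fake pucks update both players' UI and the leaderboard, clear fakes and reset the puck, gated by a one-second cooldown.
; CheckWin ends the match at the GameInstance goal count, then shows keyboards in two-player or reloads AirHockeyMain.
; Timelines animate goal, cube and material changes for Splunk.
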(event `self.ReceiveBeginPlay`
  ;[1 1 1] Begin
  (`KismetSystemLibrary.Delay` 0.2)
  (bind _returnvalue (`GameplayStatics.GetActorOfClass` "/Game/Blueprints/BP_AirhockeyPawn.BP_AirhockeyPawn_C"))
  (set `self.As BP Airhockey Pawn` _returnvalue)
  (bind _returnvalue_2 (`GameplayStatics.GetActorOfClass` "/Game/Blueprints/BP_Puck.BP_Puck_C"))
  (set `self.PuckRef` _returnvalue_2)
  (bind _returnvalue_3 (`PrimitiveComponent.CreateDynamicMaterialInstance` (`self.PlayerGoalMesh`) 0 "/Game/Materials/GradientGoals_Inst.GradientGoals_Inst" "None"))
  (set `self.PlayerGoalMatRef` _returnvalue_3)
  (bind _returnvalue_4 (`PrimitiveComponent.CreateDynamicMaterialInstance` (`self.EnemyGoalMesh`) 0 "/Game/Materials/GradientGoals_Inst.GradientGoals_Inst" "None"))
  (set `self.EnemyGoalMatRef` _returnvalue_4)
  (bind _asair_hockey_game_instance (cast `/Game/Blueprints/AirHockeyGameInstance` (`GameplayStatics.GetGameInstance`)))
  (set `self.As Air Hockey Game Instance` _asair_hockey_game_instance))

(event `/Game/Blueprints/BI_GamestartCisco.CiscoGameStarted`
  ;[1 1 1] Begin
  (`SceneComponent.SetHiddenInGame` (`self.PlayerGoalMesh`) false false)
  (`SceneComponent.SetHiddenInGame` (`self.EnemyGoalMesh`) false false)
  (bind (_direction _newtrack_0) (`Timeline|scale up` :!via `PlayFromStart`)
    (:`Update`
      (`SceneComponent.SetWorldScale3D` (`self.PlayerGoalMesh`) (`KismetMathLibrary.VLerp` (0.0 0.0 0.0) (1.0 1.0 1.0) _newtrack_0))
      (`SceneComponent.SetWorldScale3D` (`self.EnemyGoalMesh`) (`KismetMathLibrary.VLerp` (0.0 0.0 0.0) (1.0 1.0 1.0) _newtrack_0))
      (`KismetSystemLibrary.PrintString` "Hello"))))

(event `SplunkByP1`
  ;[0 0.2982 1] Splunk
  (bind (_direction _newtrack_0) (`Timeline|Timeline` :!via `PlayFromStart`)
    (:`Update`
      (`SceneComponent.SetRelativeScale3D` (`self.EnemyGoal`) (`KismetMathLibrary.VLerp` (1.0 1.0 1.0) (1.7 1.7 1.7) _newtrack_0))
      (`SceneComponent.SetRelativeScale3D` (`self.EnemyGoalMesh`) (`KismetMathLibrary.VLerp` (1.0 1.0 1.0) (1.7 1.7 1.7) _newtrack_0))
      (`SceneComponent.SetRelativeScale3D` (`self.Cube3`) (`KismetMathLibrary.VLerp` (1.0 1.0 1.0) (0.515 1.0 1.0) _newtrack_0))
      (`SceneComponent.SetRelativeScale3D` (`self.Cube2`) (`KismetMathLibrary.VLerp` (1.0 1.0 1.0) (0.515 1.0 1.0) _newtrack_0))
      (`SceneComponent.SetRelativeScale3D` (`self.PlayerGoal`) (`KismetMathLibrary.VLerp` (1.0 1.0 1.0) (0.5 0.5 0.5) _newtrack_0))
      (`SceneComponent.SetRelativeScale3D` (`self.PlayerGoalMesh`) (`KismetMathLibrary.VLerp` (1.0 1.0 1.0) (0.5 0.5 0.5) _newtrack_0))
      (`SceneComponent.SetRelativeScale3D` (`self.Cube`) (`KismetMathLibrary.VLerp` (1.0 1.0 1.0) (1.4 1.0 1.0) _newtrack_0))
      (`SceneComponent.SetRelativeScale3D` (`self.Cube1`) (`KismetMathLibrary.VLerp` (1.0 1.0 1.0) (1.4 1.0 1.0) _newtrack_0))
      (bind _returnvalue (`KismetMathLibrary.Lerp` 0.0 1.0 _newtrack_0))
      (`MaterialInstanceDynamic.SetScalarParameterValue` (`self.PlayerGoalMatRef`) "Ratio" _returnvalue)
      (`MaterialInstanceDynamic.SetScalarParameterValue` (`self.EnemyGoalMatRef`) "Ratio" _returnvalue)
      (set `self.P1UsedSplunk` true))))

(event `/Game/Blueprints/BI_GamestartCisco.DestroyPowerP1`
  ;[0 0.2982 1] Splunk
  (if (`self.P1UsedSplunk`)
    (bind (_direction _newtrack_0) (`Timeline|Timeline_0` :!via `ReverseFromEnd`)
      (:`Update`
        (`SceneComponent.SetRelativeScale3D` (`self.EnemyGoal`) (`KismetMathLibrary.VLerp` (1.0 1.0 1.0) (1.7 1.7 1.7) _newtrack_0))
        (`SceneComponent.SetRelativeScale3D` (`self.EnemyGoalMesh`) (`KismetMathLibrary.VLerp` (1.0 1.0 1.0) (1.7 1.7 1.7) _newtrack_0))
        (`SceneComponent.SetRelativeScale3D` (`self.Cube3`) (`KismetMathLibrary.VLerp` (1.0 1.0 1.0) (0.515 1.0 1.0) _newtrack_0))
        (`SceneComponent.SetRelativeScale3D` (`self.Cube2`) (`KismetMathLibrary.VLerp` (1.0 1.0 1.0) (0.515 1.0 1.0) _newtrack_0))
        (`SceneComponent.SetRelativeScale3D` (`self.PlayerGoal`) (`KismetMathLibrary.VLerp` (1.0 1.0 1.0) (0.5 0.5 0.5) _newtrack_0))
        (`SceneComponent.SetRelativeScale3D` (`self.PlayerGoalMesh`) (`KismetMathLibrary.VLerp` (1.0 1.0 1.0) (0.5 0.5 0.5) _newtrack_0))
        (`SceneComponent.SetRelativeScale3D` (`self.Cube`) (`KismetMathLibrary.VLerp` (1.0 1.0 1.0) (1.4 1.0 1.0) _newtrack_0))
        (`SceneComponent.SetRelativeScale3D` (`self.Cube1`) (`KismetMathLibrary.VLerp` (1.0 1.0 1.0) (1.4 1.0 1.0) _newtrack_0))
        (bind _returnvalue (`KismetMathLibrary.Lerp` 0.0 1.0 _newtrack_0))
        (`MaterialInstanceDynamic.SetScalarParameterValue` (`self.PlayerGoalMatRef`) "Ratio" _returnvalue)
        (`MaterialInstanceDynamic.SetScalarParameterValue` (`self.EnemyGoalMatRef`) "Ratio" _returnvalue)
        (set `self.P1UsedSplunk` false)))))

(event `SplunkByP2`
  ;[0 0.2982 1] Splunk
  (bind (_direction _newtrack_0) (`Timeline|Timeline_1` :!via `PlayFromStart`)
    (:`Update`
      (`SceneComponent.SetRelativeScale3D` (`self.PlayerGoal`) (`KismetMathLibrary.VLerp` (1.0 1.0 1.0) (1.7 1.7 1.7) _newtrack_0))
      (`SceneComponent.SetRelativeScale3D` (`self.PlayerGoalMesh`) (`KismetMathLibrary.VLerp` (1.0 1.0 1.0) (1.7 1.7 1.7) _newtrack_0))
      (`SceneComponent.SetRelativeScale3D` (`self.Cube`) (`KismetMathLibrary.VLerp` (1.0 1.0 1.0) (0.515 1.0 1.0) _newtrack_0))
      (`SceneComponent.SetRelativeScale3D` (`self.Cube1`) (`KismetMathLibrary.VLerp` (1.0 1.0 1.0) (0.515 1.0 1.0) _newtrack_0))
      (`SceneComponent.SetRelativeScale3D` (`self.EnemyGoal`) (`KismetMathLibrary.VLerp` (1.0 1.0 1.0) (0.5 0.5 0.5) _newtrack_0))
      (`SceneComponent.SetRelativeScale3D` (`self.EnemyGoalMesh`) (`KismetMathLibrary.VLerp` (1.0 1.0 1.0) (0.5 0.5 0.5) _newtrack_0))
      (`SceneComponent.SetRelativeScale3D` (`self.Cube3`) (`KismetMathLibrary.VLerp` (1.0 1.0 1.0) (1.4 1.0 1.0) _newtrack_0))
      (`SceneComponent.SetRelativeScale3D` (`self.Cube2`) (`KismetMathLibrary.VLerp` (1.0 1.0 1.0) (1.4 1.0 1.0) _newtrack_0))
      (bind _returnvalue (`KismetMathLibrary.Lerp` 0.0 1.0 _newtrack_0))
      (`MaterialInstanceDynamic.SetScalarParameterValue` (`self.PlayerGoalMatRef`) "Ratio" _returnvalue)
      (`MaterialInstanceDynamic.SetScalarParameterValue` (`self.EnemyGoalMatRef`) "Ratio" _returnvalue)
      (set `self.P2UsedSplunk` true))))

(event `/Game/Blueprints/BI_GamestartCisco.DestroyPowerP2`
  ;[0 0.2982 1] Splunk
  (if (`self.P2UsedSplunk`)
    (bind (_direction _newtrack_0) (`Timeline|Timeline_2` :!via `ReverseFromEnd`)
      (:`Update`
        (`SceneComponent.SetRelativeScale3D` (`self.PlayerGoal`) (`KismetMathLibrary.VLerp` (1.0 1.0 1.0) (1.7 1.7 1.7) _newtrack_0))
        (`SceneComponent.SetRelativeScale3D` (`self.PlayerGoalMesh`) (`KismetMathLibrary.VLerp` (1.0 1.0 1.0) (1.7 1.7 1.7) _newtrack_0))
        (`SceneComponent.SetRelativeScale3D` (`self.Cube`) (`KismetMathLibrary.VLerp` (1.0 1.0 1.0) (0.515 1.0 1.0) _newtrack_0))
        (`SceneComponent.SetRelativeScale3D` (`self.Cube1`) (`KismetMathLibrary.VLerp` (1.0 1.0 1.0) (0.515 1.0 1.0) _newtrack_0))
        (`SceneComponent.SetRelativeScale3D` (`self.EnemyGoal`) (`KismetMathLibrary.VLerp` (1.0 1.0 1.0) (0.5 0.5 0.5) _newtrack_0))
        (`SceneComponent.SetRelativeScale3D` (`self.EnemyGoalMesh`) (`KismetMathLibrary.VLerp` (1.0 1.0 1.0) (0.5 0.5 0.5) _newtrack_0))
        (`SceneComponent.SetRelativeScale3D` (`self.Cube3`) (`KismetMathLibrary.VLerp` (1.0 1.0 1.0) (1.4 1.0 1.0) _newtrack_0))
        (`SceneComponent.SetRelativeScale3D` (`self.Cube2`) (`KismetMathLibrary.VLerp` (1.0 1.0 1.0) (1.4 1.0 1.0) _newtrack_0))
        (bind _returnvalue (`KismetMathLibrary.Lerp` 0.0 1.0 _newtrack_0))
        (`MaterialInstanceDynamic.SetScalarParameterValue` (`self.PlayerGoalMatRef`) "Ratio" _returnvalue)
        (`MaterialInstanceDynamic.SetScalarParameterValue` (`self.EnemyGoalMatRef`) "Ratio" _returnvalue)
        (set `self.P2UsedSplunk` false)))))

(event `self.PlayerGoal.OnComponentBeginOverlap`
  (params (OverlappedComponent :type "PrimitiveComponent Object Reference") (OtherActor :type "Actor Object Reference") (OtherComp :type "PrimitiveComponent Object Reference") (OtherBodyIndex :type Integer) (bFromSweep :type Boolean) (SweepResult :type "HitResult Structure (by ref)"))
  (bind _as_bp_airhockey_pawn (`self.As BP Airhockey Pawn`))
  (bind _as_bp_airhockey_pawn_2 (`self.As BP Airhockey Pawn`))
  (bind _puckref (`self.PuckRef`))
  (bind _puckref_2 (`self.PuckRef`))
  ;[1 0.1994 0] Score Mechanic
  (if (not (`self.HasScoredRecently`))
    (set `self.HasScoredRecently` true)
    (if (== OtherActor "/Game/Blueprints/BP_FakePucksForP1.BP_FakePucksForP1")
      (bind _result (`/Engine/EditorBlueprintResources/StandardMacros.IncrementInt` (`self.Your Score`))
        (:`  `
          (set `self.Your Score` _result)
          (`/Game/Widget/WB_ScoreUI_P1.Update Score` (`/Game/Widget/WB_PlayerBaseUIP1.WB_ScoreUI` (`/Game/Blueprints/BP_AirhockeyPawn.UIRefP1` _as_bp_airhockey_pawn)) (`self.Your Score`) (`self.Enemy Score`))
          (`/Game/Widget/WB_ScoreUI_P2.Update Score` (`/Game/Widget/WB_PlayerBaseUIP2.WB_ScoreUI` (`/Game/Blueprints/BP_AirhockeyPawn.UIRefP2` _as_bp_airhockey_pawn)) (`self.Enemy Score`) (`self.Your Score`))
          (`/Game/Widget/WB_LeadboardUI.UpdateLeaderboardScore` (`/Game/Blueprints/BP_AirhockeyPawn.LeaderboardUIRef` _as_bp_airhockey_pawn) (`self.Your Score`) (`self.Enemy Score`))
          (bind _outactors (`GameplayStatics.GetAllActorsOfClass` "/Game/Blueprints/BP_FakePucksForP2.BP_FakePucksForP2_C"))
          (for _array_element _outactors
            (`/Game/Blueprints/BP_FakePucksForP2.Destroy P2 Fakes` _array_element))
          (switch `int` (`/Game/Blueprints/BP_AirhockeyPawn.PlayerCount` (`self.As BP Airhockey Pawn`))
            (:`1`
              (`/Game/Blueprints/BP_Puck.ResetPuckSP` _puckref))
            (:`2`
              (`/Game/Blueprints/BP_Puck.ResetPuckToP1` _puckref)))
          (`self.CheckWin`)
          (`KismetSystemLibrary.Delay` 1.0)
          (set `self.HasScoredRecently` false)
          (`self.GoalWasScored`)))
      (elif (== OtherActor (`self.PuckRef`))
        (bind _result_2 (`/Engine/EditorBlueprintResources/StandardMacros.IncrementInt` (`self.Enemy Score`))
          (:`  `
            (set `self.Enemy Score` _result_2)
            (`/Game/Widget/WB_ScoreUI_P1.Update Score` (`/Game/Widget/WB_PlayerBaseUIP1.WB_ScoreUI` (`/Game/Blueprints/BP_AirhockeyPawn.UIRefP1` _as_bp_airhockey_pawn_2)) (`self.Your Score`) (`self.Enemy Score`))
            (`/Game/Widget/WB_ScoreUI_P2.Update Score` (`/Game/Widget/WB_PlayerBaseUIP2.WB_ScoreUI` (`/Game/Blueprints/BP_AirhockeyPawn.UIRefP2` _as_bp_airhockey_pawn_2)) (`self.Enemy Score`) (`self.Your Score`))
            (`/Game/Widget/WB_LeadboardUI.UpdateLeaderboardScore` (`/Game/Blueprints/BP_AirhockeyPawn.LeaderboardUIRef` _as_bp_airhockey_pawn_2) (`self.Your Score`) (`self.Enemy Score`))
            (bind _outactors_2 (`GameplayStatics.GetAllActorsOfClass` "/Game/Blueprints/BP_FakePucksForP2.BP_FakePucksForP2_C"))
            (for _array_element_2 _outactors_2
              (`/Game/Blueprints/BP_FakePucksForP2.Destroy P2 Fakes` _array_element_2))
            (switch `int` (`/Game/Blueprints/BP_AirhockeyPawn.PlayerCount` (`self.As BP Airhockey Pawn`))
              (:`1`
                (`/Game/Blueprints/BP_Puck.ResetPuckSP` _puckref_2))
              (:`2`
                (`/Game/Blueprints/BP_Puck.ResetPuckToP1` _puckref_2)))
            (`self.CheckWin`)
            (`KismetSystemLibrary.Delay` 1.0)
            (set `self.HasScoredRecently` false)
            (`self.GoalWasScored`)))
        (else
          (set `self.HasScoredRecently` false))))))

(event `self.EnemyGoal.OnComponentBeginOverlap`
  (params (OverlappedComponent :type "PrimitiveComponent Object Reference") (OtherActor :type "Actor Object Reference") (OtherComp :type "PrimitiveComponent Object Reference") (OtherBodyIndex :type Integer) (bFromSweep :type Boolean) (SweepResult :type "HitResult Structure (by ref)"))
  (bind _as_bp_airhockey_pawn (`self.As BP Airhockey Pawn`))
  (bind _puckref (`self.PuckRef`))
  (bind _as_bp_airhockey_pawn_2 (`self.As BP Airhockey Pawn`))
  (bind _puckref_2 (`self.PuckRef`))
  ;[1 0.1994 0] Score Mechanic
  (if (not (`self.HasScoredRecently`))
    (set `self.HasScoredRecently` true)
    (if (== OtherActor "/Game/Blueprints/BP_FakePucksForP2.BP_FakePucksForP2")
      (bind _result (`/Engine/EditorBlueprintResources/StandardMacros.IncrementInt` (`self.Your Score`))
        (:`  `
          (set `self.Your Score` _result)
          (`/Game/Widget/WB_ScoreUI_P1.Update Score` (`/Game/Widget/WB_PlayerBaseUIP1.WB_ScoreUI` (`/Game/Blueprints/BP_AirhockeyPawn.UIRefP1` _as_bp_airhockey_pawn)) (`self.Your Score`) (`self.Enemy Score`))
          (`/Game/Widget/WB_ScoreUI_P2.Update Score` (`/Game/Widget/WB_PlayerBaseUIP2.WB_ScoreUI` (`/Game/Blueprints/BP_AirhockeyPawn.UIRefP2` _as_bp_airhockey_pawn)) (`self.Enemy Score`) (`self.Your Score`))
          (`/Game/Widget/WB_LeadboardUI.UpdateLeaderboardScore` (`/Game/Blueprints/BP_AirhockeyPawn.LeaderboardUIRef` _as_bp_airhockey_pawn) (`self.Your Score`) (`self.Enemy Score`))
          (bind _outactors (`GameplayStatics.GetAllActorsOfClass` "/Game/Blueprints/BP_FakePucksForP1.BP_FakePucksForP1_C"))
          (for _array_element _outactors
            (`/Game/Blueprints/BP_FakePucksForP1.Destroy P1 Fakes` _array_element))
          (switch `int` (`/Game/Blueprints/BP_AirhockeyPawn.PlayerCount` (`self.As BP Airhockey Pawn`))
            (:`1`
              (`/Game/Blueprints/BP_Puck.ResetPuckSP` _puckref))
            (:`2`
              (`/Game/Blueprints/BP_Puck.ResetPuckToP2` _puckref)))
          (`self.CheckWin`)
          (`KismetSystemLibrary.Delay` 1.0)
          (set `self.HasScoredRecently` false)
          (`self.GoalWasScored`)))
      (elif (== OtherActor (`self.PuckRef`))
        (bind _result_2 (`/Engine/EditorBlueprintResources/StandardMacros.IncrementInt` (`self.Your Score`))
          (:`  `
            (set `self.Your Score` _result_2)
            (`/Game/Widget/WB_ScoreUI_P1.Update Score` (`/Game/Widget/WB_PlayerBaseUIP1.WB_ScoreUI` (`/Game/Blueprints/BP_AirhockeyPawn.UIRefP1` _as_bp_airhockey_pawn_2)) (`self.Your Score`) (`self.Enemy Score`))
            (`/Game/Widget/WB_ScoreUI_P2.Update Score` (`/Game/Widget/WB_PlayerBaseUIP2.WB_ScoreUI` (`/Game/Blueprints/BP_AirhockeyPawn.UIRefP2` _as_bp_airhockey_pawn_2)) (`self.Enemy Score`) (`self.Your Score`))
            (`/Game/Widget/WB_LeadboardUI.UpdateLeaderboardScore` (`/Game/Blueprints/BP_AirhockeyPawn.LeaderboardUIRef` _as_bp_airhockey_pawn_2) (`self.Your Score`) (`self.Enemy Score`))
            (bind _outactors_2 (`GameplayStatics.GetAllActorsOfClass` "/Game/Blueprints/BP_FakePucksForP1.BP_FakePucksForP1_C"))
            (for _array_element_2 _outactors_2
              (`/Game/Blueprints/BP_FakePucksForP1.Destroy P1 Fakes` _array_element_2))
            (switch `int` (`/Game/Blueprints/BP_AirhockeyPawn.PlayerCount` (`self.As BP Airhockey Pawn`))
              (:`1`
                (`/Game/Blueprints/BP_Puck.ResetPuckSP` _puckref_2))
              (:`2`
                (`/Game/Blueprints/BP_Puck.ResetPuckToP2` _puckref_2)))
            (`self.CheckWin`)
            (`KismetSystemLibrary.Delay` 1.0)
            (set `self.HasScoredRecently` false)
            (`self.GoalWasScored`)))
        (else
          (set `self.HasScoredRecently` false))))))

(event `CheckWin`
  (bind _istwoplayer (`/Game/Blueprints/BP_AirhockeyPawn.IsTwoPlayer` (`self.As BP Airhockey Pawn`)))
  (bind _uirefp2 (`/Game/Blueprints/BP_AirhockeyPawn.UIRefP2` (`self.As BP Airhockey Pawn`)))
  (bind _numberofgoals (`/Game/Blueprints/AirHockeyGameInstance.NumberOfGoals` (`self.As Air Hockey Game Instance`)))
  (bind _leaderboarduiref (`/Game/Blueprints/BP_AirhockeyPawn.LeaderboardUIRef` (`self.As BP Airhockey Pawn`)))
  (bind _uirefp1 (`/Game/Blueprints/BP_AirhockeyPawn.UIRefP1` (`self.As BP Airhockey Pawn`)))
  ;[0.6433 1 0] Check Win
  (if (or (>= (`self.Your Score`) _numberofgoals) (>= (`self.Enemy Score`) _numberofgoals))
    (if (> (`self.Your Score`) (`self.Enemy Score`))
      (`KismetSystemLibrary.PrintString` "p1 wins")
      (set `/Game/Blueprints/BP_AirhockeyPawn.IsAllowedToMove` false (`self.As BP Airhockey Pawn`))
      (`/Game/Blueprints/AirHockeyGameInstance.StopCountGameTime` (`self.As Air Hockey Game Instance`))
      (`/Game/Widget/WB_PlayerBaseUIP1.P1 Win` _uirefp1)
      (if _istwoplayer
        (`/Game/Widget/WB_LeadboardUI.ShowLeaderboard` _leaderboarduiref)
        (`KismetSystemLibrary.Delay` 10.0)
        (`/Game/Widget/WB_PlayerBaseUIP1.KeyboardVisible` _uirefp1)
        (`/Game/Widget/WB_PlayerBaseUIP2.KeyboardVisible` (`/Game/Blueprints/BP_AirhockeyPawn.UIRefP2` (`self.As BP Airhockey Pawn`)))
        (else
          (`/Game/Widget/WB_LeadboardUI.ShowLeaderboard` _leaderboarduiref)
          (`KismetSystemLibrary.Delay` 10.0)
          (`MultiWindowExtensionSubsystem.KB_MWE_CloseAll` (subsystem `MultiWindowExtensionSubsystem`))
          (`GameplayStatics.OpenLevel` "AirHockeyMain")))
      (else
        (`KismetSystemLibrary.PrintString` "p2 wins")
        (set `/Game/Blueprints/BP_AirhockeyPawn.IsAllowedToMove` false (`self.As BP Airhockey Pawn`))
        (`/Game/Blueprints/AirHockeyGameInstance.StopCountGameTime` (`self.As Air Hockey Game Instance`))
        (`/Game/Widget/WB_PlayerBaseUIP2.P2 Win` _uirefp2)
        (if _istwoplayer
          (`/Game/Widget/WB_LeadboardUI.ShowLeaderboard` _leaderboarduiref)
          (`KismetSystemLibrary.Delay` 10.0)
          (`/Game/Widget/WB_PlayerBaseUIP2.KeyboardVisible` _uirefp2)
          (`/Game/Widget/WB_PlayerBaseUIP1.KeyboardVisible` (`/Game/Blueprints/BP_AirhockeyPawn.UIRefP1` (`self.As BP Airhockey Pawn`)))
          (else
            (`/Game/Widget/WB_LeadboardUI.ShowLeaderboard` _leaderboarduiref)
            (`KismetSystemLibrary.Delay` 10.0)
            (`MultiWindowExtensionSubsystem.KB_MWE_CloseAll` (subsystem `MultiWindowExtensionSubsystem`))
            (`GameplayStatics.OpenLevel` "AirHockeyMain")))))))

(fn `UserConstructionScript`)