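; BP_Table is the air hockey table actor that detects when the puck enters either of its two goals.
; Each goal component's begin-overlap event casts the other actor to BP_Puk and hides the puck's static mesh.
; After a short delay it reloads the match by opening the AirHockeyMain level, with no scoring in this Blueprint.
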(event `self.Goal1.OnComponentBeginOverlap`
  (params (OverlappedComponent :type "PrimitiveComponent Object Reference") (OtherActor :type "Actor Object Reference") (OtherComp :type "PrimitiveComponent Object Reference") (OtherBodyIndex :type Integer) (bFromSweep :type Boolean) (SweepResult :type "HitResult Structure (by ref)"))
  (bind _asbp_puk (cast `/Game/Blueprints/BP_Puk` OtherActor))
  (`SceneComponent.SetHiddenInGame` (`/Game/Blueprints/BP_Puk.StaticMesh` _asbp_puk) true false)
  (`KismetSystemLibrary.Delay` 0.5)
  (`GameplayStatics.OpenLevel` "AirHockeyMain"))

(event `self.Goal.OnComponentBeginOverlap`
  (params (OverlappedComponent :type "PrimitiveComponent Object Reference") (OtherActor :type "Actor Object Reference") (OtherComp :type "PrimitiveComponent Object Reference") (OtherBodyIndex :type Integer) (bFromSweep :type Boolean) (SweepResult :type "HitResult Structure (by ref)"))
  (bind _asbp_puk (cast `/Game/Blueprints/BP_Puk` OtherActor))
  (`SceneComponent.SetHiddenInGame` (`/Game/Blueprints/BP_Puk.StaticMesh` _asbp_puk) true false)
  (`KismetSystemLibrary.Delay` 0.5)
  (`GameplayStatics.OpenLevel` "AirHockeyMain"))

(fn `UserConstructionScript`)