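; BP_FakePucksForP2 is a decoy puck, apparently spawned by Player 2's power, with a constantly spinning Paper sprite.
; It scales up from zero on BeginPlay, then enables physics simulation on its mesh.
; Hitting Player 1's paddle plays a random sound, shrinks the puck and destroys it after a short delay.
; Two custom events, DestroyPowerP2 and DestroyP2Fakes, trigger the same shrink-and-destroy through another timeline.
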(event `self.ReceiveBeginPlay`
  (bind (_direction _newtrack_0) (`Timeline|Timeline_0`)
    (:`Update`
      (`self.SetActorRelativeScale3D` (`KismetMathLibrary.VLerp` (0.0 0.0 0.0) (0.2 0.2 0.2) _newtrack_0)))
    (:`Finished`
      (`PrimitiveComponent.SetSimulatePhysics` (`self.StaticMesh`) true))))

(event `/Game/Blueprints/BI_GamestartCisco.DestroyPowerP2`
  (bind (_direction _newtrack_0) (`Timeline|Timeline` :!via `PlayFromStart` :!label _label)
    (:`Update`
      (`self.SetActorRelativeScale3D` (`KismetMathLibrary.VLerp` (0.2 0.2 0.2) (0.0 0.0 0.0) _newtrack_0))
      (`KismetSystemLibrary.Delay` 0.25)
      (`self.K2_DestroyActor`))))

(event `Destroy P2 Fakes`
  (goto _label :!via `PlayFromStart`))

(event `self.StaticMesh.OnComponentHit`
  (params (HitComponent :type "PrimitiveComponent Object Reference") (OtherActor :type "Actor Object Reference") (OtherComp :type "PrimitiveComponent Object Reference") (NormalImpulse :type "Vector Structure") (Hit :type "HitResult Structure (by ref)"))
  (cast `/Game/Blueprints/BP_PaddleP1` OtherActor)
  (`GameplayStatics.PlaySoundAtLocation` (`|GetArrayItem` (`self.Sound`) (`KismetMathLibrary.RandomIntegerInRange` 0 3)) (0.0 0.0 0.0) (struct) 1.0 1.0 0.0 null null null null)
  (bind (_direction _newtrack_0) (`Timeline|Timeline_1` :!via `PlayFromStart`)
    (:`Update`
      (`self.SetActorRelativeScale3D` (`KismetMathLibrary.VLerp` (0.2 0.2 0.2) (0.0 0.0 0.0) _newtrack_0))
      (`KismetSystemLibrary.Delay` 0.25)
      (`self.K2_DestroyActor`))))

(event `self.ReceiveTick`
  (params (DeltaSeconds :type "Float (single-precision)"))
  (bind _output_get (set `self.New Rotation Z (Yaw)` (+ (`self.New Rotation Z (Yaw)`) 1.0)))
  (`SceneComponent.K2_SetWorldRotation` (`self.PaperSprite`) (`KismetMathLibrary.MakeRotator` 90.0 0.0 _output_get) false false))

(fn `UserConstructionScript`)