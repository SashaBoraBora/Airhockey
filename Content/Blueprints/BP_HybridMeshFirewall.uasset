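; BP_HybridMeshFirewall is a firewall power actor in an air hockey game, made up of attached segment actors.
; On BeginPlay it counts those segments and binds to the DestroyPower dispatcher on the player pawn's active-power widget.
; That event starts a timeline that scales the segments toward zero, and the firewall destroys itself after a short delay.
; Decrement lowers the segment count and destroys the firewall when it reaches zero.
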(event `self.ReceiveBeginPlay`
  (bind _asbp_airhockey_pawn (cast `/Game/Blueprints/BP_AirhockeyPawn` (`GameplayStatics.GetPlayerPawn` 0)))
  (set `self.As BP Airhockey Pawn` _asbp_airhockey_pawn)
  (set `self.RemainingSegments` (`KismetArrayLibrary.Array_Length` (`self.GetAttachedActors` true)))
  (add `/Game/Widget/WB_ActivePowerP1.DestroyPower` (`/Game/Widget/WB_PlayerBaseUIP1.WB_ActivePower` (`/Game/Blueprints/BP_AirhockeyPawn.UIRefP1` (`self.As BP Airhockey Pawn`))) (delegate `DestroyPower_Event`)))

(event `DestroyPower_Event`
  (bind (_direction _newtrack_0) (`Timeline|Timeline`)
    (:`Update`
      (for _array_element (`self.GetAttachedActors` true)
        (`self.SetActorRelativeScale3D` _array_element (`KismetMathLibrary.VLerp` (1.0 1.0 1.0) (0.0 0.0 0.0) _newtrack_0))
        (`KismetSystemLibrary.Delay` 0.25)
        (`self.K2_DestroyActor`)))))

(event `Decrement`
  (`/Engine/EditorBlueprintResources/StandardMacros.DecrementInt` (`self.RemainingSegments`)
    (:`  `
      (if (== (`self.RemainingSegments`) 0)
        (`KismetSystemLibrary.PrintString` "Destroyed")
        (`self.K2_DestroyActor`)
        (else
          (`KismetSystemLibrary.PrintString` "NotDestroyed"))))))

(fn `UserConstructionScript`)