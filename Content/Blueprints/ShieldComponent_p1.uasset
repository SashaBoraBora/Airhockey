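; Player 1 shield piece actor that is destroyed when a BP_Puck overlaps its box.
; After a short delay, a timeline scales the mesh down toward zero.
; A delay chained from the timeline's update, rather than its finish, then calls Decrement on the parent BP_P1_HybridMeshFirewall and destroys the actor.
; If the attach parent is not that firewall, the actor is not destroyed.
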(event `self.ReceiveBeginPlay`
  (`PrimitiveComponent.SetMaterial` (`self.StaticMesh`) 0 (`self.Material_0`))
  (`PrimitiveComponent.SetMaterial` (`self.StaticMesh`) 1 (`self.Material_1`)))

(event `self.Box.OnComponentBeginOverlap`
  (params (OverlappedComponent :type "PrimitiveComponent Object Reference") (OtherActor :type "Actor Object Reference") (OtherComp :type "PrimitiveComponent Object Reference") (OtherBodyIndex :type Integer) (bFromSweep :type Boolean) (SweepResult :type "HitResult Structure (by ref)"))
  (cast `/Game/Blueprints/BP_Puck` OtherActor)
  (`KismetSystemLibrary.Delay` 0.2)
  (bind (_direction _newtrack_0) (`Timeline|ScaleDown`)
    (:`Update`
      (`SceneComponent.SetRelativeScale3D` (`self.StaticMesh`) (`KismetMathLibrary.VLerp` (1.0 1.0 1.0) (0.0 0.0 0.0) _newtrack_0))
      (`KismetSystemLibrary.Delay` 1.0)
      (bind _asbp_p1_hybrid_mesh_firewall (cast `/Game/Blueprints/BP_P1_HybridMeshFirewall` (`self.GetAttachParentActor`)))
      (`/Game/Blueprints/BP_P1_HybridMeshFirewall.Decrement` _asbp_p1_hybrid_mesh_firewall)
      (`self.K2_DestroyActor`))))

(fn `UserConstructionScript`)