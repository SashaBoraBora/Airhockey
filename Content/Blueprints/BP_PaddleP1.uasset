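; Player 1's air hockey paddle, which follows touch input and strikes the puck.
; Unless the game instance uses markers, Tick checks touches while movement is allowed, keeps those deprojecting to positive world Y, line-traces them and sweeps the mesh there at fixed height.
; Puck hits play a random sound, adding a special impulse while the ZTNA power is active.
; Enable and destroy events toggle that power on both paddle and puck.
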(event `self.ReceiveBeginPlay`
  (bind _returnvalue (`GameplayStatics.GetActorOfClass` "/Game/Blueprints/BP_Puck.BP_Puck_C"))
  (set `self.PuckRef` _returnvalue)
  (bind _asbp_airhockey_pawn (cast `/Game/Blueprints/BP_AirhockeyPawn` (`GameplayStatics.GetPlayerPawn` 0)))
  (set `self.As BP Airhockey Pawn` _asbp_airhockey_pawn)
  (bind _asair_hockey_game_instance (cast `/Game/Blueprints/AirHockeyGameInstance` (`GameplayStatics.GetGameInstance`)))
  (set `self.As Air Hockey Game Instance` _asair_hockey_game_instance))

(event `/Game/Blueprints/BI_GamestartCisco.DestroyPowerP1`
  (set `self.ZTNAActiveP1` false)
  (set `/Game/Blueprints/BP_Puck.ZTNAAllowedP1` false (`self.PuckRef`)))

(event `EnableZTNA`
  (set `self.ZTNAActiveP1` true)
  (set `/Game/Blueprints/BP_Puck.ZTNAAllowedP1` true (`self.PuckRef`)))

(event `self.StaticMesh.OnComponentHit`
  (params (HitComponent :type "PrimitiveComponent Object Reference") (OtherActor :type "Actor Object Reference") (OtherComp :type "PrimitiveComponent Object Reference") (NormalImpulse :type "Vector Structure") (Hit :type "HitResult Structure (by ref)"))
  (if (`self.ZTNAActiveP1`)
    (bind _asbp_puck (cast `/Game/Blueprints/BP_Puck` OtherActor))
    (`GameplayStatics.PlaySoundAtLocation` (`|GetArrayItem` (`self.Sound`) (`KismetMathLibrary.RandomIntegerInRange` 0 3)) (0.0 0.0 0.0) (struct) 1.0 1.0 0.0 null null null null)
    (`/Game/Blueprints/BP_Puck.AddImpulseZTNAP1` _asbp_puck)
    (else
      (cast `/Game/Blueprints/BP_Puck` OtherActor)
      (`GameplayStatics.PlaySoundAtLocation` (`|GetArrayItem` (`self.Sound`) (`KismetMathLibrary.RandomIntegerInRange` 0 3)) (0.0 0.0 0.0) (struct) 1.0 1.0 0.0 null null null null))))

(event `self.ReceiveTick`
  (params (DeltaSeconds :type "Float (single-precision)"))
  (bind _returnvalue (`GameplayStatics.GetPlayerController` 0))
  (bind (_worldlocation _worlddirection) (`PlayerController.DeprojectScreenPositionToWorld` (`GameplayStatics.GetPlayerController` 0) (`self.Location X`) (`self.Location Y`)))
  (if (`/Game/Blueprints/AirHockeyGameInstance.UseMarker` (`self.As Air Hockey Game Instance`))
    _
    (elif (`/Game/Blueprints/BP_AirhockeyPawn.IsAllowedToMove` (`self.As BP Airhockey Pawn`))
      (for _array_element (`self.Finger Index`)
        (bind (_locationx _locationy) (`PlayerController.GetInputTouchState` _returnvalue _array_element))
        (if (> (.y (`PlayerController.DeprojectScreenPositionToWorld` _returnvalue _locationx _locationy)) 0.0)
          (set `self.Location Y` _locationy)
          (set `self.Location X` _locationx)
          (bind _outhit (`KismetSystemLibrary.LineTraceSingle` _worldlocation (+ _worldlocation (* _worlddirection 10000.0)) "TraceTypeQuery1"))
          (`SceneComponent.K2_SetWorldLocation` (`self.StaticMesh`) (`KismetMathLibrary.MakeVector` (.x (`.Location` (`GameplayStatics.BreakHitResult` _outhit))) (.y (`.Location` (`GameplayStatics.BreakHitResult` _outhit))) 10.0) true false))))))

(fn `UserConstructionScript`)