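; BP_BaseBumper is a bumper actor that knocks a BP_Puck away when it enters the bumper's Box trigger.
; On overlap it plays a GeometryCache animation and applies an impulse scaled by PlungerStrength, directed along the difference between the puck and plunger relative locations.
; A DoOnce gate with a 0.2-second delayed reset debounces repeat hits, and BeginPlay assigns a material to the plunger mesh.
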(event `self.ReceiveBeginPlay`
  (`PrimitiveComponent.SetMaterial` (`self.PlungerStaticMesh`) 1 (`self.Material`)))

(event `self.Box.OnComponentBeginOverlap`
  (params (OverlappedComponent :type "PrimitiveComponent Object Reference") (OtherActor :type "Actor Object Reference") (OtherComp :type "PrimitiveComponent Object Reference") (OtherBodyIndex :type Integer) (bFromSweep :type Boolean) (SweepResult :type "HitResult Structure (by ref)"))
  (bind _asbp_puck (cast `/Game/Blueprints/BP_Puck` OtherActor))
  (`/Engine/EditorBlueprintResources/StandardMacros.DoOnce` false :!label _label
    (:`Completed`
      (`GeometryCacheComponent.PlayFromStart` (`self.Geometry Cache`))
      (bind _puck (`/Game/Blueprints/BP_Puck.Puck` _asbp_puck))
      (`PrimitiveComponent.AddImpulse` _puck (* (`KismetMathLibrary.Normal` (- (`SceneComponent.RelativeLocation` _puck) (`SceneComponent.RelativeLocation` (`self.PlungerStaticMesh`)))) (`self.PlungerStrength`)) "None" false)
      (`KismetSystemLibrary.Delay` 0.2)
      (goto _label :!via `Reset`))))

(fn `UserConstructionScript`)