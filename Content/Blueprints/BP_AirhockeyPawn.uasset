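; Air hockey pawn that creates both player HUDs and a leaderboard in a separate window, then handles starting one- or two-player games.
; Start events notify BI_GamestartCisco actors, place paddles and enable movement after a delay; two-player mode requires two counted players and spawns the second paddle.
; Disconnected logic would position paddles by mouse or by the circumcenter of three traced touches per player; Tick is empty.
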(event Custom|StartTwoPlayerMode
  ;[1 0 0.3732] StartTwoPlayerMode
  (if (>= (Variables|Default|GetPlayerCount) 2)
    (bind _returnvalue (AddComponent|AddChildActorComponent false (Math|Transform|MakeTransform "0.000000,-170.000000,10.000000" "0, 0, 0" "4.000000,4.000000,4.000000")))
    (Variables|Default|SetPlayer2Paddle _returnvalue)
    (bind _outactors (Actor|GetAllActorswithInterface "/Game/Blueprints/BI_GamestartCisco.BI_GamestartCisco_C"))
    (for _array_element _outactors
      (Class|BIGamestartCisco|CiscoGameStarted(Message) _array_element)
      (Development|SetHiddeninGame (Variables|Default|GetPlayer2Paddle) false false)
      (Transformation|SetWorldLocation (Variables|Default|GetPlayer2Paddle) "0.000000,170.000000,10.000000" true false)
      (Utilities|FlowControl|Delay 1.0)
      (Variables|Default|SetIsAllowedToMove true))))

(event Custom|StartSinglePlayerMode
  ;[0 0.5673 1] StartSinglePlayerMode
  (bind _outactors (Actor|GetAllActorswithInterface "/Game/Blueprints/BI_GamestartCisco.BI_GamestartCisco_C"))
  (for _array_element _outactors
    (Class|BIGamestartCisco|CiscoGameStarted(Message) _array_element)
    (Development|SetHiddeninGame (Variables|Default|GetPlayer1Paddle) false false)
    (Transformation|SetWorldLocation (Variables|Default|GetPlayer1Paddle) "0.000000,170.000000,10.000000" true false)
    (Utilities|FlowControl|Delay 1.0)
    (Variables|Default|SetIsAllowedToMove true)))

(event Custom|CheckPlayerCount
  ;[1 0 0.3732] StartTwoPlayerMode
  (bind _result (Math|Integer|IncrementInt (Variables|Default|GetPlayerCount))
    (:%20%20
      (Variables|Default|SetPlayerCount _result))))

(event EventTick
  (params (DeltaSeconds :type Float%20%28single-precision%29))
  ;[0.8042 1 0] Touch Tracker
)

(event EventBeginPlay
  ;[1 1 1] Begin
  (bind _returnvalue (Actor|GetActorOfClass "/Game/Blueprints/BP_Puck.BP_Puck_C"))
  (Variables|Default|SetPukRef _returnvalue)
  (bind _returnvalue_2 (UserInterface|CreateWidget "/Game/Widget/WB_PlayerBaseUIP1.WB_PlayerBaseUIP1_C"))
  (bind _output_get (Variables|Default|SetUIRefP1 _returnvalue_2))
  (UserInterface|Viewport|AddtoViewport _output_get 0)
  (bind _returnvalue_3 (UserInterface|CreateWidget "/Game/Widget/WB_PlayerBaseUIP2.WB_PlayerBaseUIP2_C"))
  (bind _output_get_2 (Variables|Default|SetUIRefP2 _returnvalue_3))
  (UserInterface|Viewport|AddtoViewport _output_get_2 0)
  (bind _returnvalue_4 (UserInterface|CreateWidget "/Game/Widget/WB_LeadboardUI.WB_LeadboardUI_C"))
  (bind _returnvalue_5 (Class|MultiWindowExtensionSubsystem|KBMWECreate (Subsystems|GetMultiWindowExtensionSubsystem) (Utilities|GetClass _returnvalue_4) (Variables|Default|GetWindow%20Settings)))
  (Variables|Default|SetLeaderboardUIRef _returnvalue_5)
  (Variables|/Script/Engine.PlayerController|SetbShowMouseCursor (Game|GetPlayerController 0) true))

(event Input|KeyboardEvents|DebugKey2
  (params (Key :type Key%20Structure :default "None") (ActionValue :type Input%20Action%20Value%20Structure))
  ;[1 1 1] Begin
  (:Pressed
    (Widget|RemovefromParent (stale EventBeginPlay _output_get))))

(event Input|KeyboardEvents|Escape
  (params (Key :type Key%20Structure :default "None"))
  (:Pressed
    (EventDispatchers|UnbindallEventsfromOnClosed (Subsystems|GetMultiWindowExtensionSubsystem))))

(fn ConstructionScript)