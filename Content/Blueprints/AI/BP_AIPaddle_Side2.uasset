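; AI opponent paddle for air hockey that chases the puck on its negative-Y half and otherwise retreats home.
; A Tick-driven state machine switches from Idle to Chase when the puck is slow and within bounds; paddle hits and goals force Defend.
; Chase uses VectorSlerpNormals on world positions, while Defend lerps home, both with swept moves.
; Cooldown is never entered, and its timer resets on every call.
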(event `self.ReceiveBeginPlay`
  (bind _returnvalue (`GameplayStatics.GetActorOfClass` "/Game/Blueprints/BP_Puck.BP_Puck_C"))
  (set `self.PukRef` _returnvalue)
  (bind _asbp_airhockey_pawn (cast `/Game/Blueprints/BP_AirhockeyPawn` (`GameplayStatics.GetPlayerPawn` 0)))
  (set `self.As BP Airhockey Pawn` _asbp_airhockey_pawn)
  (bind _returnvalue_2 (`GameplayStatics.GetActorOfClass` "/Game/Blueprints/BP_TableGoals.BP_TableGoals_C"))
  (set `self.GoalRef` _returnvalue_2)
  (add `/Game/Blueprints/BP_TableGoals.GoalWasScored` (`self.GoalRef`) (delegate `GoalWasScored_Event`)))

(event `GoalWasScored_Event`
  (set `self.AI_State` "NewEnumerator2"))

(event `self.paddle.OnComponentHit`
  (params (HitComponent :type "PrimitiveComponent Object Reference") (OtherActor :type "Actor Object Reference") (OtherComp :type "PrimitiveComponent Object Reference") (NormalImpulse :type "Vector Structure") (Hit :type "HitResult Structure (by ref)"))
  (cast `/Game/Blueprints/BP_Puck` OtherActor)
  (set `self.AI_State` "NewEnumerator2"))

(event `self.ReceiveTick`
  (params (DeltaSeconds :type "Float (single-precision)"))
  (switch `/Game/Blueprints/E_AIState` (`self.AI_State`)
    (:`NewEnumerator0`
      (bind _returnvalue (`self.Idle`))
      (if _returnvalue
        (set `self.AI_State` "NewEnumerator1")
        (else
          (set `self.AI_State` "NewEnumerator2"))))
    (:`NewEnumerator1`
      (`self.Chase`))
    (:`NewEnumerator2`
      (`self.Defend`)
      (set `self.AI_State` "NewEnumerator0"))
    (:`NewEnumerator3`
      (`self.Cooldown`)
      (set `self.AI_State` "NewEnumerator0"))))

(fn `Chase`
  (locals (NewLocalVar :type "Vector Structure" :default (0.0 0.0 0.0)))
  (bind _paddle (`self.paddle`))
  (bind (_returnvalue_x _returnvalue_y) (`KismetMathLibrary.BreakVector` (`self.K2_GetActorLocation` (`self.PukRef`))))
  (bind (_returnvalue_x_2 _returnvalue_y_2) (`KismetMathLibrary.BreakVector` (`self.K2_GetActorLocation` (`self.PukRef`))))
  (bind (_returnvalue_x_3 _returnvalue_y_3) (`KismetMathLibrary.BreakVector` (`SceneComponent.K2_GetComponentLocation` (`self.paddle`))))
  (bind (_returnvalue_x_4 _returnvalue_y_4) (`KismetMathLibrary.BreakVector` (`KismetMathLibrary.Vector_SlerpNormals` (`SceneComponent.K2_GetComponentLocation` _paddle) (`self.K2_GetActorLocation` (`self.PukRef`)) 0.1)))
  (if (>= _returnvalue_y 0.0)
    (`self.Defend` :!label _label)
    (elif (< _returnvalue_y_2 _returnvalue_y_3)
      (goto _label)
      (else
        (`SceneComponent.K2_SetWorldLocation` _paddle (`KismetMathLibrary.MakeVector` _returnvalue_x_4 _returnvalue_y_4 12.0) true false)))))

(fn `Cooldown`
  (returns (CooldownEnd :type Boolean))
  (`self.Defend`)
  (set `self.CDTimer` 2.0)
  (bind _output_get (set `self.CDTimer` (- (`self.CDTimer`) (`GameplayStatics.GetWorldDeltaSeconds`))))
  (bind _returnvalue (<= _output_get 0.0))
  (if _returnvalue
    (return _returnvalue)))

(fn `Defend`
  (bind (_returnvalue_x _returnvalue_y) (`KismetMathLibrary.BreakVector` (`KismetMathLibrary.VLerp` (`SceneComponent.K2_GetComponentLocation` (`self.paddle`)) (`|GetArrayItem` (`self.PaddleHomeLocation`)) 0.1)))
  (`SceneComponent.K2_SetWorldLocation` (`self.paddle`) (`KismetMathLibrary.MakeVector` _returnvalue_x _returnvalue_y 12.0) true false))

(fn `Idle`
  (returns (ReturnValue :type Boolean))
  (bind _pukref (`self.PukRef`))
  (bind (_returnvalue_x _returnvalue_y) (`KismetMathLibrary.BreakVector` (`self.K2_GetActorLocation` _pukref)))
  (return (and (< _returnvalue_y 0.0) (< _returnvalue_x 100.0) (> _returnvalue_x -100.0) (< _returnvalue_x 190.0) (not (> (`KismetMathLibrary.VSize` (`self.GetVelocity` _pukref)) (`self.PuckSpeedThreshold`))))))

(fn `UserConstructionScript`)