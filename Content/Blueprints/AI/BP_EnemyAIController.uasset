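; AI controller that drives the enemy paddle against the puck in what appears to be an air-hockey style game.
; BeginPlay caches the paddle and puck actors.
; Each Tick eases the paddle toward the puck's X/Y at a fixed height, or back to a home position when the puck is hidden or on the positive-Y side.
; Movement uses interpolated, unswept SetActorLocation calls, with no pathfinding.
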(event `self.ReceiveBeginPlay`
  (bind _returnvalue (`GameplayStatics.GetActorOfClass` "/Game/Blueprints/AI/BP_EnemyPaddle.BP_EnemyPaddle_C"))
  (set `self.EnemyPaddleRef` _returnvalue)
  (bind _returnvalue_2 (`GameplayStatics.GetActorOfClass` "/Game/Blueprints/BP_Puk.BP_Puk_C"))
  (set `self.Puk Ref` _returnvalue_2))

(event `self.ReceiveTick`
  (params (DeltaSeconds :type "Float (single-precision)"))
  (bind _staticmesh (`/Game/Blueprints/BP_Puk.StaticMesh` (`self.Puk Ref`)))
  (bind (_returnvalue_x _returnvalue_y) (`KismetMathLibrary.BreakVector` (`SceneComponent.K2_GetComponentLocation` _staticmesh)))
  (if (or (> _returnvalue_y 0.0) (not (`SceneComponent.IsVisible` _staticmesh)))
    (`self.K2_SetActorLocation` (`self.EnemyPaddleRef`) (`KismetMathLibrary.VInterpTo` (`SceneComponent.K2_GetComponentLocation` (`/Game/Blueprints/AI/BP_EnemyPaddle.StaticMesh` (`self.EnemyPaddleRef`))) (0.0 -170.0 10.2) DeltaSeconds 5.0) false false)
    (else
      (`self.K2_SetActorLocation` (`self.EnemyPaddleRef`) (`KismetMathLibrary.MakeVector` (`KismetMathLibrary.FInterpTo` (.x (`SceneComponent.K2_GetComponentLocation` (`/Game/Blueprints/AI/BP_EnemyPaddle.StaticMesh` (`self.EnemyPaddleRef`)))) (.x (`SceneComponent.K2_GetComponentLocation` (`/Game/Blueprints/BP_Puk.StaticMesh` (`self.Puk Ref`)))) DeltaSeconds 7.0) (`KismetMathLibrary.FInterpTo` (.y (`SceneComponent.K2_GetComponentLocation` (`/Game/Blueprints/AI/BP_EnemyPaddle.StaticMesh` (`self.EnemyPaddleRef`)))) (.y (`SceneComponent.K2_GetComponentLocation` (`/Game/Blueprints/BP_Puk.StaticMesh` (`self.Puk Ref`)))) DeltaSeconds 7.0) 10.2) false false))))

(fn `UserConstructionScript`)