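; BP_XDR is an air hockey power actor that removes itself when the active power's DestroyPower event fires.
; On BeginPlay it binds to that dispatcher on the first player pawn's P1 active-power widget.
; The event plays a timeline that lerps each directly attached actor's relative scale toward zero.
; A short delay inside that update loop leads to the actor destroying itself.
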(event `self.ReceiveBeginPlay`
  (bind _asbp_airhockey_pawn (cast `/Game/Blueprints/BP_AirhockeyPawn` (`GameplayStatics.GetPlayerPawn` 0)))
  (bind _output_get (set `self.As BP Airhockey Pawn` _asbp_airhockey_pawn))
  (add `/Game/Widget/WB_ActivePower.DestroyPower` (`/Game/Widget/WB_PlayerBaseUIP1.WB_ActivePower` (`/Game/Blueprints/BP_AirhockeyPawn.UIRefP1` _output_get)) (delegate `DestroyPower_Event`)))

(event `DestroyPower_Event`
  (bind (_direction _newtrack_0) (`Timeline|Timeline`)
    (:`Update`
      (for _array_element (`self.GetAttachedActors` true)
        (`self.SetActorRelativeScale3D` _array_element (`KismetMathLibrary.VLerp` (1.0 1.0 1.0) (0.0 0.0 0.0) _newtrack_0))
        (`KismetSystemLibrary.Delay` 0.25)
        (`self.K2_DestroyActor`)))))

(fn `UserConstructionScript`)