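; BP_ShieldPickup is an air hockey shield power-up actor made of attached segment actors.
; On BeginPlay it counts its directly attached actors as remaining segments and binds to the DestroyPower dispatcher on the player pawn's pickup-use widget.
; It destroys itself when that dispatcher fires or when calls to its Decrement event bring the segment count to zero, printing debug messages on each decrement.
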(event `self.ReceiveBeginPlay`
  (bind _asbp_airhockey_pawn (cast `/Game/Blueprints/BP_AirhockeyPawn` (`GameplayStatics.GetPlayerPawn` 0)))
  (set `self.As BP Airhockey Pawn` _asbp_airhockey_pawn)
  (set `self.RemainingSegments` (`KismetArrayLibrary.Array_Length` (`self.GetAttachedActors` true)))
  (add `/Game/Widget/WB_UsePickUPNew.DestroyPower` (`/Game/Widget/WB_PlayerBaseUI.WB_UsePickUPnew` (`/Game/Blueprints/BP_AirhockeyPawn.UIRef` (`self.As BP Airhockey Pawn`))) (delegate `DestroyPower_Event`)))

(event `DestroyPower_Event`
  (`self.K2_DestroyActor`))

(event `Decrement`
  (`/Engine/EditorBlueprintResources/StandardMacros.DecrementInt` (`self.RemainingSegments`)
    (:`  `
      (if (== (`self.RemainingSegments`) 0)
        (`KismetSystemLibrary.PrintString` "Destroyed")
        (`self.K2_DestroyActor`)
        (else
          (`KismetSystemLibrary.PrintString` "NotDestroyed"))))))

(fn `UserConstructionScript`)